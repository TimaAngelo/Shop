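; PC player character for furniture shopping and room design, with movement, a HUD and a room-creation widget.
; E runs a server/multicast-named event chain into a camera trace that opens furniture editing or messages other interactables.
; Favorites from the game instance fill a HUD picker that spawns a material-swapped preview.
; Tick moves the preview along camera traces, R rotates it through a gate, and left click spawns the final copy.
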(event Custom|EventAddFavorit
  ;[1 1 1] LoadDate
  (bind _asbp_base_game_instance (Utilities|Casting|CastToBP_BaseGameInstance (Game|GetGameInstance)))
  (bind _output_get (Variables|/Game/SHOP/Blueprint/Characters/ComputerCharacter/Component/BP_TotalComponentInfo.BP_TotalComponentInfo_C|SetFurniturActor (Variables|Default|GetBP_TotalComponentInfo) (Variables|/Game/SHOP/Blueprint/Core/BP_BaseGameInstance.BP_BaseGameInstance_C|GetFavoritFurniturActor _asbp_base_game_instance)))
  (for _array_element _output_get
    (Default|EventCreateFavorit (Variables|/Game/SHOP/Blueprint/Widget/HUD/BP_HUDPC.BP_HUDPC_C|GetWG_EditFavorit (Variables|Widget|GetHUD)) _array_element)))

(event EventBeginPlay
  ;[1 1 1] HudCreate
  (bind _returnvalue (UserInterface|CreateWidget "/Game/SHOP/Blueprint/Widget/HUD/BP_HUDPC.BP_HUDPC_C"))
  (bind _output_get (Variables|Widget|SetHUD _returnvalue))
  (UserInterface|Viewport|AddtoViewport _output_get 0)
  (CallFunction|EventAddFavorit))

(event Input|AxisEvents|InputAxisLookUp
  (params (AxisValue :type Float%20%28single-precision%29))
  ;[1 1 1] MouseController
  (if (not (Variables|Default|GetIsEditMode))
    (Pawn|Input|AddControllerPitchInput AxisValue)))

(event Input|AxisEvents|InputAxisTurn
  (params (AxisValue :type Float%20%28single-precision%29))
  ;[1 1 1] MouseController
  (if (not (Variables|Default|GetIsEditMode))
    (Pawn|Input|AddControllerYawInput AxisValue)))

(event Input|AxisEvents|InputAxisMoveForward
  (params (AxisValue :type Float%20%28single-precision%29))
  ;[1 1 1] Movement
  (Pawn|Input|AddMovementInput (Math|Vector|GetForwardVector (Math|Rotator|MakeRotator 0.0 0.0 (.Yaw (Math|Rotator|BreakRotator (Pawn|GetControlRotation :!class /Script/Engine.Pawn))))) AxisValue false))

(event Input|AxisEvents|InputAxisMoveRight
  (params (AxisValue :type Float%20%28single-precision%29))
  ;[1 1 1] Movement
  (Pawn|Input|AddMovementInput (Math|Vector|GetRightVector (Math|Rotator|MakeRotator 0.0 0.0 (.Yaw (Math|Rotator|BreakRotator (Pawn|GetControlRotation :!class /Script/Engine.Pawn))))) AxisValue false))

(event Custom|Interact_Server
  ;[1 1 1] Replication
  (CallFunction|InteractMulticast))

(event Custom|Interact_Multicast
  ;[1 1 1] Replication
  (CallFunction|EditMode))

(event Custom|UnEditMode
  ;[1 1 1] OffEditMode
  (Widget|SetVisibility (Variables|/Game/SHOP/Blueprint/Widget/HUD/BP_HUDPC.BP_HUDPC_C|GetBP_EditMenuWidget (Variables|Widget|GetHUD)) "Hidden")
  (Variables|/Script/Engine.PlayerController|SetbShowMouseCursor (Game|GetPlayerController 0) false)
  (Pawn|Components|CharacterMovement|SetMovementMode (Variables|Character|GetCharacterMovement) "MOVE_Walking" 0)
  (if (Variables|Default|GetIsButMode)
    (Development|SetHiddeninGame (Variables|Character|GetMesh) false false)
    (Game|Player|SetViewTargetwithBlend (Game|GetPlayerController 0) self 0.5 "VTBlend_Linear" 0.2 false)
    (Variables|Default|SetIsEditMode false)
    (else
      (Variables|Default|SetIsEditMode false))))

(event Custom|EventAcceptLocation
  ;[1 1 1] AcceptLocation
  (Game|SpawnActorfromClass (Utilities|GetClass (Variables|Default|GetCreatedFurniturPref)) (Math|Transform|MakeTransform (Variables|Default|GetAcceptLocation) (Variables|Default|GetRotateFurn) "1,1,1") "Undefined" 0 0)
  (bind _createdfurniturpref (Variables|Default|GetCreatedFurniturPref)
    (:then
      (Actor|DestroyActor _createdfurniturpref)
      (Variables|Default|SetIsPastMode false))
    (:else)))

(event Custom|EditMode
  ;[1 1 1] Replication
  (CallFunction|ChekFunction)
  (Variables|Default|SetIsEditMode true))

(event EventTick
  (params (DeltaSeconds :type Float%20%28single-precision%29))
  ;[1 1 1] Past Tick
  (Utilities|FlowControl|Sequence
    (:then_0
      (Utilities|FlowControl|Gate true
        (:Exit
          (Variables|Default|SetRotateFurn (Math|Rotator|MakeRotator (.roll (Transformation|GetActorRotation (stale Input|KeyboardEvents|R _createdfurniturpref))) (.pitch (Transformation|GetActorRotation (stale Input|KeyboardEvents|R _createdfurniturpref))) (+ (.yaw (Transformation|GetActorRotation (stale Input|KeyboardEvents|R _createdfurniturpref))) 1.0))))))
    (:then_1
      (CallFunction|GetLocationFurn))))

(event EventSpawnActor
  (params (FurnitureClass :type BP%20Base%20Furniture%20Class%20Reference))
  (bind _returnvalue (Game|GetPlayerCameraManager 0))
  (bind _returnvalue_2 (Transformation|GetActorLocation _returnvalue))
  ;[1 1 1] SpawnActor
  (if (Variables|Default|GetIsPastMode)
    (bind _outhit (Collision|LineTraceByChannel _returnvalue_2 (+ _returnvalue_2 (* (Transformation|GetActorForwardVector _returnvalue) 1e+03)) "TraceTypeQuery1" false 0 "None"))
    (bind _returnvalue_3 (Game|SpawnActorfromClass FurnitureClass (Math|Transform|MakeTransform (.Location (Collision|BreakHitResult _outhit)) (Variables|Default|GetRotateFurn) "1,1,1") "Undefined" 0 0))
    (bind _output_get (Variables|Default|SetCreatedFurniturPref _returnvalue_3))
    (Rendering|Material|SetMaterial (Variables|/Game/SHOP/Blueprint/InteractActors/Furniture/BP_BaseFurniture.BP_BaseFurniture_C|GetStaticMesh _output_get) 0 "/Engine/VREditor/UI/DiscMaterial.DiscMaterial")
    (Variables|Default|SetIsPastMode true)
    (Widget|SetVisibility (Variables|/Game/SHOP/Blueprint/Widget/HUD/BP_HUDPC.BP_HUDPC_C|GetWG_EditFavorit (Variables|Widget|GetHUD)) "Hidden")
    (Variables|/Script/Engine.PlayerController|SetbShowMouseCursor (Game|GetPlayerController 0) false)
    (Variables|Default|SetIsEditMode false)))

(event Input|KeyboardEvents|C
  (params (Key :type Key%20Structure :default "None"))
  ;[1 1 1] GetPastMode
  (:Pressed
    (if (Utilities|Enum|Equal(Enum) (Widget|GetVisibility (Variables|/Game/SHOP/Blueprint/Widget/HUD/BP_HUDPC.BP_HUDPC_C|GetWG_EditFavorit (Variables|Widget|GetHUD))) "Visible")
      (Widget|SetVisibility (Variables|/Game/SHOP/Blueprint/Widget/HUD/BP_HUDPC.BP_HUDPC_C|GetWG_EditFavorit (Variables|Widget|GetHUD)) "Hidden")
      (Variables|Default|SetIsPastMode true)
      (Variables|/Script/Engine.PlayerController|SetbShowMouseCursor (Game|GetPlayerController 0) false)
      (Variables|Default|SetIsEditMode true)
      (else
        (Widget|SetVisibility (Variables|/Game/SHOP/Blueprint/Widget/HUD/BP_HUDPC.BP_HUDPC_C|GetWG_EditFavorit (Variables|Widget|GetHUD)) "Visible")
        (Variables|Default|SetIsPastMode true)
        (Variables|/Script/Engine.PlayerController|SetbShowMouseCursor (Game|GetPlayerController 0) true)
        (Variables|Default|SetIsEditMode true)))))

(event Input|MouseEvents|LeftMouseButton
  (params (Key :type Key%20Structure :default "None"))
  ;[1 1 1] PastAccept
  (:Pressed
    (if (Variables|Default|GetIsPastMode)
      (CallFunction|EventAcceptLocation))))

(event Input|KeyboardEvents|B
  (params (Key :type Key%20Structure :default "None"))
  ;[1 1 1] OpenRoom
  (:Pressed
    (bind _returnvalue (UserInterface|CreateWidget "/Game/SHOP/Blueprint/Widget/HUD/BP_CreateRoom.BP_CreateRoom_C"))
    (bind _output_get (Variables|Widget|SetCreateRommWidget _returnvalue))
    (UserInterface|Viewport|AddtoViewport _output_get 0)
    (Variables|/Script/Engine.PlayerController|SetbShowMouseCursor (Game|GetPlayerController 0) true)
    (Variables|Default|SetIsEditMode true)
    (Default|EventSaveFavorit (Variables|Default|GetBP_TotalComponentInfo))))

(event Input|KeyboardEvents|E
  (params (Key :type Key%20Structure :default "None"))
  ;[1 1 1] Interact Button (E)
  (:Pressed
    (if (Variables|Default|GetIsEditMode)
      (CallFunction|UnEditMode)
      (else
        (CallFunction|InteractServer)))))

(event Input|KeyboardEvents|R
  (params (Key :type Key%20Structure :default "None"))
  (:Pressed
    (bind _createdfurniturpref (Variables|Default|GetCreatedFurniturPref)
      (:then
        (Utilities|FlowControl|Gate true) ; enters at Open
      )
      (:else)))
  (:Released
    (Utilities|FlowControl|Gate true) ; enters at Close
  ))

(fn ConstructionScript)

(fn ChekFunction
  (bind _camera (Variables|Default|GetCamera))
  (bind _returnvalue (Transformation|GetWorldLocation _camera))
  (bind (_outhit _returnvalue_2) (Collision|LineTraceByChannel _returnvalue (+ _returnvalue (* (Math|Vector|GetForwardVector _camera) 5e+02)) "TraceTypeQuery1" false 0 "ForDuration"))
  (if _returnvalue_2
    (if (Utilities|DoesObjectImplementInterface (.HitActor (Collision|BreakHitResult _outhit)) "/Game/SHOP/Blueprint/Characters/ComputerCharacter/Interface/BP_Interact.BP_Interact_C")
      (if (.bSuccess (Utilities|Casting|CastToBP_BaseFurniture (.HitActor (Collision|BreakHitResult _outhit))))
        (Widget|SetVisibility (Variables|/Game/SHOP/Blueprint/Widget/HUD/BP_HUDPC.BP_HUDPC_C|GetBP_EditMenuWidget (Variables|Widget|GetHUD)) "Visible")
        (bind _output_get (Variables|Interact|SetActorInteract (.AsBP%20Base%20Furniture (Utilities|Casting|CastToBP_BaseFurniture (.HitActor (Collision|BreakHitResult _outhit))))))
        (Default|GetSetting _output_get)
        (Variables|/Script/Engine.PlayerController|SetbShowMouseCursor (Game|GetPlayerController 0) true)
        (Pawn|Components|CharacterMovement|SetMovementMode (Variables|Character|GetCharacterMovement) "MOVE_None" 0)
        (if (Variables|Default|GetIsButMode)
          (Development|SetHiddeninGame (Variables|Character|GetMesh) true false)
          (Game|Player|SetViewTargetwithBlend (Game|GetPlayerController 0) (Variables|Interact|GetActorInteract) 0.5 "VTBlend_Linear" 0.0 false)
          (return)
          (else
            (return)))
        (else
          (Class|BPInteract|Interact(Message) (.HitActor (Collision|BreakHitResult _outhit)))))
      (else
        (return)))
    (else
      (return))))

(fn GetLocationFurn
  (bind _createdfurniturpref (Variables|Default|GetCreatedFurniturPref))
  (bind _camera (Variables|Default|GetCamera))
  (bind _returnvalue (Transformation|GetWorldLocation _camera))
  (if (Variables|Default|GetIsPastMode)
    (bind _outhit (Collision|LineTraceByChannel _returnvalue (+ _returnvalue (* (Math|Vector|GetForwardVector _camera) 1e+03)) "TraceTypeQuery1" false (Utilities|Array|MakeArray (Variables|Default|GetCreatedFurniturPref)) "None"))
    (if (.bblockinghit _outhit)
      (Utilities|IsValid _createdfurniturpref
        (:Is%20Valid
          (Transformation|SetActorLocationAndRotation _createdfurniturpref (.location _outhit) (Variables|Default|GetRotateFurn))
          (Variables|Default|SetAcceptLocation (.location _outhit)))))))
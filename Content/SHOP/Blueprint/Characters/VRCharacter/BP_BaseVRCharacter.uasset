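; Base VR character for a furniture shop game, with axis movement, teleport locomotion and a HUD.
; BeginPlay creates the HUD widget and fills its favorites editor with furniture from the game instance.
; While a teleport input is held, Tick predicts an arc from the opposite hand's controller and immediately teleports to upward-facing hits, drawing debug visuals.
; SelectObject is an uncalled line-trace stub.
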(event Custom|EventAddFavorit
  ;[1 1 1] LoadDate
  (bind _asbp_base_game_instance (Utilities|Casting|CastToBP_BaseGameInstance (Game|GetGameInstance)))
  (bind _output_get (Variables|/Game/SHOP/Blueprint/Characters/ComputerCharacter/Component/BP_TotalComponentInfo.BP_TotalComponentInfo_C|SetFurniturActor (Variables|Default|GetBP_TotalComponentInfo) (Variables|/Game/SHOP/Blueprint/Core/BP_BaseGameInstance.BP_BaseGameInstance_C|GetFavoritFurniturActor _asbp_base_game_instance)))
  (for _array_element _output_get
    (Default|EventCreateFavorit (Variables|/Game/SHOP/Blueprint/Widget/HUD/BP_HUDPC.BP_HUDPC_C|GetWG_EditFavorit (Variables|Default|GetHUD)) _array_element)))

(event EventBeginPlay
  ;[1 1 1] Event Begin Play
  (bind _returnvalue (UserInterface|CreateWidget "/Game/SHOP/Blueprint/Widget/HUD/BP_HUDPC.BP_HUDPC_C"))
  (Variables|Default|SetHUD _returnvalue)
  (CallFunction|EventAddFavorit))

(event EventTick
  (params (DeltaSeconds :type Float%20%28single-precision%29))
  ;[1 1 1] Event Tick
  (if (Variables|Default|GetIsTeleport)
    (CallFunction|TeleportPosition (select (Variables|Default|GetIsTeleportL) (Variables|Default|GetMotionController_R) (Variables|Default|GetMotionController_L)))))

(event Input|ActionEvents|InputActionTeleportL
  (params (Key :type Key%20Structure :default "None"))
  ;[1 1 1] TeleportMove_L
  (:Pressed
    (Variables|Default|SetIsTeleport true)
    (Variables|Default|SetIsTeleportL true)
    (Development|PrintString "LL"))
  (:Released
    (Variables|Default|SetIsTeleport false)
    (Variables|Default|SetIsTeleportL false)))

(event Input|ActionEvents|InputActionTeleportR
  (params (Key :type Key%20Structure :default "None"))
  ;[1 1 1] TeleportMove_R
  (:Pressed
    (Variables|Default|SetIsTeleport true)
    (Variables|Default|SetIsTeleportL false)
    (Development|PrintString "RR"))
  (:Released
    (Variables|Default|SetIsTeleport false)))

(event Input|AxisEvents|InputAxisMoveForward
  (params (AxisValue :type Float%20%28single-precision%29))
  ;[1 1 1] Movement
  (Pawn|Input|AddMovementInput (Math|Vector|GetForwardVector (Math|Rotator|MakeRotator 0.0 0.0 (.Yaw (Math|Rotator|BreakRotator (Pawn|GetControlRotation :!class /Script/Engine.Pawn))))) AxisValue false))

(event Input|AxisEvents|InputAxisMoveRight
  (params (AxisValue :type Float%20%28single-precision%29))
  ;[1 1 1] Movement
  (Pawn|Input|AddMovementInput (Math|Vector|GetRightVector (Math|Rotator|MakeRotator 0.0 0.0 (.Yaw (Math|Rotator|BreakRotator (Pawn|GetControlRotation :!class /Script/Engine.Pawn))))) AxisValue false))

(fn ConstructionScript)

(fn TeleportPosition
  (params (Target :type Scene%20Component%20Object%20Reference))
  (bind (_outhit _outpathpositions _outlasttracedestination _returnvalue) (Class|GameplayStatics|BlueprintPredictProjectilePathbyObjectType (Transformation|GetWorldLocation Target) (* (Math|Vector|GetForwardVector (Transformation|GetWorldRotation Target)) (Variables|Default|GetTeleportLenght)) true 1e+01 (Utilities|Array|MakeArray "ObjectTypeQuery1" "ObjectTypeQuery2") false 0 "ForOneFrame" 0.0 2e+01))
  (if _returnvalue
    (if (> (.Z (Math|Vector|BreakVector (.ImpactNormal (Collision|BreakHitResult _outhit)))) 0.0)
      (bind _output_get (Variables|Default|SetTeleportLocation (.ImpactPoint (Collision|BreakHitResult _outhit))))
      (Class|KismetSystemLibrary|DrawDebugCylinder _output_get (+ _output_get 2e+01) 5e+01 12 "(R=0.065776,G=0.000000,B=1.000000,A=1.000000)" 0.0 0.0)
      (Transformation|Teleport (Variables|Default|GetTeleportLocation) (Transformation|GetActorRotation)))))

(fn SelectObject
  (params (Target :type Scene%20Component%20Object%20Reference))
  (bind _returnvalue (Transformation|GetWorldLocation Target))
  (bind (_outhit _returnvalue_2) (Collision|LineTraceByChannel _returnvalue (+ _returnvalue (* (Math|Vector|GetForwardVector (Transformation|GetWorldRotation Target)) (Variables|Default|GetTeleportLenght))) "TraceTypeQuery1" false 0 "None"))
  (if _returnvalue_2
    _))
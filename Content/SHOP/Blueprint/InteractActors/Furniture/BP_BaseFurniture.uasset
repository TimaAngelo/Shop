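; Base furniture actor for the shop that the player can customize and mark as a favorite.
; It caches the player character on BeginPlay and passes its materials, colors, name, type and size to the HUD edit menu.
; Material changes create a dynamic instance on the mesh, and color changes set its "Col" parameter.
; Favoriting adds or re-adds the actor to the character's furniture list and updates the favorites widget with its material.
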(event Custom|GetSetting
  (bind _as_bp_base_character_pc (Variables|Default|GetAs%20BP%20Base%20Character%20PC))
  (bind _hud (Variables|/Game/SHOP/Blueprint/Characters/ComputerCharacter/BP_BaseCharacterPC.BP_BaseCharacterPC_C|GetHUD _as_bp_base_character_pc))
  ;[1 1 1] GenerateSettings
  (Utilities|IsValid _hud
    (:Is%20Valid
      (Default|Generate (Variables|/Game/SHOP/Blueprint/Widget/HUD/BP_HUDPC.BP_HUDPC_C|GetBP_EditMenuWidget _hud) (Variables|Default|GetST_Material) (Variables|Default|GetST_Color) self (Variables|Default|GetName) (Variables|Default|GetType) (Variables|Default|GetSize)))))

(event Custom|EventSetColor
  (params (Color :type Color%20Structure))
  ;[1 1 1] SwitchColor
  (Rendering|Material|SetVectorParameterValueonMaterials (Variables|Default|GetStaticMesh) "Col" (Math|Vector|MakeVector (Math|Conversions|ToFloat(Byte) (.r Color)) (Math|Conversions|ToFloat(Byte) (.g Color)) (Math|Conversions|ToFloat(Byte) (.b Color)))))

(event Custom|EventSetMaterial
  (params (Material :type Material%20Interface%20Object%20Reference))
  ;[1 1 1] SetMaterial
  (bind _returnvalue (Rendering|Material|CreateDynamicMaterialInstance Material "Instance" "Transient" :!class /Script/Engine.KismetMaterialLibrary))
  (Rendering|Material|SetMaterial (Variables|Default|GetStaticMesh) 0 _returnvalue))

(event Custom|EventAddFavorit
  (bind _self self)
  (bind _as_bp_base_character_pc (Variables|Default|GetAs%20BP%20Base%20Character%20PC))
  (bind _staticmesh (Variables|Default|GetStaticMesh))
  (bind _as_bp_base_character_pc_2 (Variables|Default|GetAs%20BP%20Base%20Character%20PC))
  (bind _returnvalue (Rendering|Material|GetMaterial _staticmesh 0))
  (bind _hud (Variables|/Game/SHOP/Blueprint/Characters/ComputerCharacter/BP_BaseCharacterPC.BP_BaseCharacterPC_C|GetHUD _as_bp_base_character_pc))
  (bind _bp_totalcomponentinfo (Variables|/Game/SHOP/Blueprint/Characters/ComputerCharacter/BP_BaseCharacterPC.BP_BaseCharacterPC_C|GetBP_TotalComponentInfo _as_bp_base_character_pc_2))
  (bind _furnituractor (Variables|/Game/SHOP/Blueprint/Characters/ComputerCharacter/Component/BP_TotalComponentInfo.BP_TotalComponentInfo_C|GetFurniturActor _bp_totalcomponentinfo))
  (bind _wg_editfavorit (Variables|/Game/SHOP/Blueprint/Widget/HUD/BP_HUDPC.BP_HUDPC_C|GetWG_EditFavorit _hud))
  ;[1 1 1] Add favorit
  (if (!= _self (Utilities|Array|Get(acopy) _furnituractor (Utilities|Array|FindItem _furnituractor _self)))
    (Utilities|Array|AddUnique _furnituractor self)
    (Default|EventCreateFavorit _wg_editfavorit self)
    (Variables|/Game/SHOP/Blueprint/Widget/NewWidget/WG_EditFavorit.WG_EditFavorit_C|SetMaterial _wg_editfavorit _returnvalue)
    (else
      (Utilities|Array|RemoveItem _furnituractor (Utilities|Array|Get(acopy) _furnituractor (Utilities|Array|FindItem _furnituractor _self)))
      (Utilities|Array|AddUnique _furnituractor _self)
      (Default|EventCreateFavorit _wg_editfavorit self)
      (Variables|/Game/SHOP/Blueprint/Widget/NewWidget/WG_EditFavorit.WG_EditFavorit_C|SetMaterial _wg_editfavorit _returnvalue))))

(event EventBeginPlay
  ;[1 1 1] Begin Play
  (bind _asbp_base_character_pc (Utilities|Casting|CastToBP_BaseCharacterPC (Game|GetPlayerCharacter 0)))
  (Variables|Default|SetAs%20BP%20Base%20Character%20PC _asbp_base_character_pc))

(fn ConstructionScript)